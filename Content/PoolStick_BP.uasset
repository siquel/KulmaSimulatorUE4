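; Pool cue Blueprint that lets the player aim around the cue ball and strike it.
; At BeginPlay it moves itself to the CueBall's location.
; The Turn axis adds controller yaw and copies the control rotation onto the root component.
; Left click applies a fixed-strength force to the ball's Sphere opposite the Keppi component's forward vector, with the vertical component zeroed.
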(event `self.ReceiveBeginPlay`
  (`self.K2_SetActorLocation` (`self.K2_GetActorLocation` (`self.CueBall`))))

(event `self.ReceiveActorBeginOverlap`
  (params (OtherActor :type "Actor Object Reference")))

(event `self.ReceiveTick`
  (params (DeltaSeconds :type "Float (single-precision)")))

(event `Key|LeftMouseButton`
  (params (Key :type "Key Structure" :default "AnyKey"))
  (:`Pressed`
    (`PrimitiveComponent.AddForce` (`/Game/FirstPerson/PoolBall.Sphere` (`self.CueBall`)) (* (`SceneComponent.GetForwardVector` (`self.keppi`)) (-100000.0 -100000.0 0.0)) "None" false)))

(event `InputAxis|Turn`
  (params (AxisValue :type "Float (single-precision)"))
  (`self.AddControllerYawInput` AxisValue)
  (`SceneComponent.K2_SetWorldRotation` (`self.DefaultSceneRoot`) (`Controller.GetControlRotation` (`GameplayStatics.GetPlayerController` 0)) false false))

(fn `UserConstructionScript`)